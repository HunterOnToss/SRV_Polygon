(event `self.ReceiveBeginPlay`
  (`self.InitializePlayer`))

(event `self.ReceiveTick`
  (params (DeltaSeconds :type "Float (single-precision)"))
  (`self.Aiming`))

(event `Key|E`
  (params (Key :type "Key Structure"))
  (:`Pressed`
    (`self.OnActorUsed`)))

(event `OnActorUsed`
  (bind _hitactor (`self.CheckItem`))
  (`/Engine/EditorBlueprintResources/StandardMacros.IsValid` _hitactor
    (:`Is Valid`
      (message `/Game/SRV_Polygon/Blueprints/Character/Interface/I_Interact.PickUp` _hitactor (`self.CharacterReference`)))))

(event `Key|RightMouseButton`
  (params (Key :type "Key Structure"))
  (:`Pressed`
    (set `self.IsAiming` true))
  (:`Released`
    (set `self.IsAiming` false)))

(event `self.InventoryManagerComponent.OnInventoryStateUpdate`
  (bind _ui_inventory (`self.UI_Inventory`))
  (`/Engine/EditorBlueprintResources/StandardMacros.IsValid` _ui_inventory
    (:`Is Valid`
      (`/Game/SRV_Polygon/Blueprints/Equipment/Items/UI/UI_Inventory.UpdateData` _ui_inventory))))

(event `Key|I`
  (params (Key :type "Key Structure"))
  (bind _ui_inventory (`self.UI_Inventory`))
  (:`Pressed`
    (`/Engine/EditorBlueprintResources/StandardMacros.IsValid` (`self.UI_Inventory`)
      (:`Is Valid`
        (`/Game/SRV_Polygon/Blueprints/Equipment/Items/UI/UI_Inventory.UpdateData` _ui_inventory)
        (`UserWidget.AddToViewport` _ui_inventory 0))
      (:`Is Not Valid`
        (bind _returnvalue (`|CreateWidget` "/Game/SRV_Polygon/Blueprints/Equipment/Items/UI/UI_Inventory.UI_Inventory_C" self))
        (bind _output_get (set `self.UI_Inventory` _returnvalue))
        (`/Game/SRV_Polygon/Blueprints/Equipment/Items/UI/UI_Inventory.SetInventoryRef` _output_get (`self.InventoryManagerComponent`))
        (`UserWidget.AddToViewport` _output_get 0)))))

(event `Key|G`
  (params (Key :type "Key Structure"))
  (bind _inventorymanagercomponent (`self.InventoryManagerComponent`))
  (bind _output (`|GetArrayItem` (`/Game/SRV_Polygon/Blueprints/Equipment/InventoryManagerComponent.InventoryStorageItems` _inventorymanagercomponent)))
  (:`Pressed`
    (`/Engine/EditorBlueprintResources/StandardMacros.IsValid` _output
      (:`Is Valid`
        (`/Game/SRV_Polygon/Blueprints/Equipment/InventoryManagerComponent.DropItemToWorld` _inventorymanagercomponent _output)))))

(event `Key|LeftMouseButton`
  (params (Key :type "Key Structure"))
  (:`Pressed`
    (set `self.IsFirePressed` true)
    (`self.Shoot`))
  (:`Released`
    (set `self.IsFirePressed` false)
    (`self.Shoot`)))

(fn `Aiming`
  (bind _followcamera (`/Game/SRV_Polygon/Blueprints/Character/BP_BaseCharacter.FollowCamera` (`self.CharacterReference`)))
  (set `CameraComponent.FieldOfView` (`KismetMathLibrary.FInterpTo` (`CameraComponent.FieldOfView` _followcamera) (`KismetMathLibrary.SelectFloat` (`self.AimFieldOfView`) (`self.StandartFieldOfView`) (`self.IsAiming`)) (`GameplayStatics.GetWorldDeltaSeconds`) (`self.AimFOVSpeed`)) _followcamera))

(fn `CheckItem`
  (returns (HitActor :type "Actor Object Reference"))
  (bind _characterreference (`self.CharacterReference`))
  (bind _followcamera (`/Game/SRV_Polygon/Blueprints/Character/BP_BaseCharacter.FollowCamera` _characterreference))
  (bind _returnvalue (`SceneComponent.K2_GetComponentLocation` _followcamera))
  (bind _outhit (`KismetSystemLibrary.LineTraceSingleForObjects` _returnvalue (+ _returnvalue (* (`KismetMathLibrary.Conv_RotatorToVector` (`SceneComponent.K2_GetComponentRotation` _followcamera)) (+ (`SpringArmComponent.TargetArmLength` (`/Game/SRV_Polygon/Blueprints/Character/BP_BaseCharacter.CameraBoom` _characterreference)) (`self.MaxCheckDistance`)))) (`|MakeArray` "ObjectTypeQuery7" "ObjectTypeQuery1" "ObjectTypeQuery2" :!type "EObjectTypeQuery Enum") false (`|MakeArray` (`self.CharacterReference`) :!type "Actor Object Reference")))
  (bind (_bblockinghit _binitialoverlap _time _distance _location _impactpoint _normal _impactnormal _physmat _hitactor) (`GameplayStatics.BreakHitResult` _outhit))
  (if (`KismetSystemLibrary.DoesImplementInterface` _hitactor "/Game/SRV_Polygon/Blueprints/Character/Interface/I_Interact.I_Interact_C")
    (return _hitactor)
    (else
      (return null))))

(fn `InitializePlayer`
  (bind _asbp_base_character (cast `/Game/SRV_Polygon/Blueprints/Character/BP_BaseCharacter` (`self.K2_GetPawn`)))
  (set `self.CharacterReference` _asbp_base_character))

(fn `Shoot`
  (bind _equipedweapon (`/Game/SRV_Polygon/Blueprints/Equipment/InventoryManagerComponent.GetCurrentEquipedWeapon` (`self.InventoryManagerComponent`)))
  (`/Engine/EditorBlueprintResources/StandardMacros.IsValid` _equipedweapon
    (:`Is Valid`
      (if (`/Game/SRV_Polygon/Blueprints/Equipment/Items/Weapons/BP_BaseWeapon.IsEquiped` _equipedweapon)
        (`/Game/SRV_Polygon/Blueprints/Equipment/Items/Weapons/BP_BaseWeapon.UseWeapon` _equipedweapon (`self.IsFirePressed`))
        (else
          (`KismetSystemLibrary.PrintString` "Weapon not Equipped"))))))

(fn `UserConstructionScript`)