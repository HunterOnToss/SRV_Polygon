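; BP_MyLibs is an equipment helper library that converts between attachment point values and socket names.
; GetSocketNameByPoint maps the left leg, right leg, spine and lower spine points to their socket names.
; GetSocketPointByName does the reverse lookup, switching on the socket name to return the matching point.
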(fn `GetSocketNameByPoint`
  (params (Point :type "/Game/SRV_Polygon/Blueprints/Equipment/E_AttachPoint Enum" :default "NewEnumerator0"))
  (returns (Name :type Name))
  (switch `/Game/SRV_Polygon/Blueprints/Equipment/E_AttachPoint` Point
    (:`NewEnumerator0`
      (return "S_Left"))
    (:`NewEnumerator1`
      (return "S_Right"))
    (:`NewEnumerator2`
      (return "S_Back"))
    (:`NewEnumerator3`
      (return "S_BackSecond"))))

(fn `GetSocketPointByName`
  (params (Name :type Name))
  (returns (Point :type "/Game/SRV_Polygon/Blueprints/Equipment/E_AttachPoint Enum"))
  (switch `name` Name
    (:`S_Left`
      (return "NewEnumerator0"))
    (:`S_Right`
      (return "NewEnumerator1"))
    (:`S_Back`
      (return "NewEnumerator2"))
    (:`S_BackSecond`
      (return "NewEnumerator3"))))