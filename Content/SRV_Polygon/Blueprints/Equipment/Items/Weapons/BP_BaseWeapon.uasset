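; Base weapon actor that handles pickup into the player's inventory, equipping and firing.
; Equip and UnEquip move it between character mesh sockets, returning it to its stored attach point.
; UseWeapon triggers Shoot, a debug-print placeholder, while Tick runs the uses-per-second cooldown and repeats auto-fire.
; A damage helper applies simple or point damage from a hit result.
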(event `self.ReceiveTick`
  (params (DeltaSeconds :type "Float (single-precision)"))
  (`parent.ReceiveTick` DeltaSeconds)
  (`self.WeaponTimer`)
  (if (and (`self.Firing`) (`self.IsAbleToUse`))
    (`self.UseWeapon` true)))

(event `AttachWeaponToCharacter`
  (params (SocketName :type Name))
  (bind _asbp_base_character (cast `/Game/SRV_Polygon/Blueprints/Character/BP_BaseCharacter` (`self.GetOwner`)))
  (bind _mesh (`Character.Mesh` _asbp_base_character))
  (if (`SceneComponent.DoesSocketExist` _mesh SocketName)
    (`self.K2_AttachToComponent` _mesh SocketName "SnapToTarget" "SnapToTarget" "KeepRelative")
    (set `self.CurrentAttachPoint` (`/Game/SRV_Polygon/Blueprints/Equipment/BP_MyLibs.GetSocketPointByName` SocketName))))

(event `Equip`
  (bind _asbp_base_character (cast `/Game/SRV_Polygon/Blueprints/Character/BP_BaseCharacter` (`self.GetOwner`)))
  (`self.K2_AttachToComponent` (`Character.Mesh` _asbp_base_character) (`self.EquipedSocketName`) "SnapToTarget" "SnapToTarget" "KeepRelative")
  (set `self.IsEquiped` true))

(event `UnEquip`
  (set `self.IsEquiped` false)
  (bind _asbp_base_character (cast `/Game/SRV_Polygon/Blueprints/Character/BP_BaseCharacter` (`self.GetOwner`)))
  (`self.K2_AttachToComponent` (`Character.Mesh` _asbp_base_character) (`/Game/SRV_Polygon/Blueprints/Equipment/BP_MyLibs.GetSocketNameByPoint` (`self.CurrentAttachPoint`)) "SnapToTarget" "SnapToTarget" "KeepRelative"))

(fn `IsAbleToUse`
  (returns (Success :type Boolean))
  (return (`self.WeaponCanBeUse?`)))

(fn `MakeDamageUseType`
  (params (DamageType :type "/Game/SRV_Polygon/Blueprints/Equipment/Items/Weapons/E_WeaponDamageType Enum" :default "E_WeaponDamageType_MAX") (Damage :type "Float (double-precision)") (Hit :type "HitResult Structure") (DamageCauser :type "Actor Object Reference"))
  (returns (Success :type Boolean))
  (locals (L_Damage :type "Float (double-precision)") (L_Hit :type "HitResult Structure") (L_DamageCauser :type "Actor Object Reference"))
  (bind (_bblockinghit _binitialoverlap _time _distance _location _impactpoint _normal _impactnormal _physmat _hitactor _hitcomponent _hitbonename _hititem _faceindex _tracestart _traceend) (`GameplayStatics.BreakHitResult` (`local.L_Hit`)))
  (bind (_bblockinghit_2 _binitialoverlap_2 _time_2 _distance_2 _location_2 _impactpoint_2 _normal_2 _impactnormal_2 _physmat_2 _hitactor_2) (`GameplayStatics.BreakHitResult` (`local.L_Hit`)))
  (set `local.L_Damage` Damage)
  (set `local.L_Hit` Hit)
  (set `local.L_DamageCauser` DamageCauser)
  (switch `/Game/SRV_Polygon/Blueprints/Equipment/Items/Weapons/E_WeaponDamageType` DamageType
    (:`NewEnumerator0`
      (`/Engine/EditorBlueprintResources/StandardMacros.IsValid` _hitactor_2
        (:`Is Valid`
          (`GameplayStatics.ApplyDamage` _hitactor_2 (`local.L_Damage`) (`self.GetInstigatorController`) (`local.L_DamageCauser`))
          (return true))
        (:`Is Not Valid`
          (return false))))
    (:`NewEnumerator1`
      (`/Engine/EditorBlueprintResources/StandardMacros.IsValid` _hitactor
        (:`Is Valid`
          (`GameplayStatics.ApplyPointDamage` _hitactor 0.0 (`KismetMathLibrary.GetDirectionUnitVector` _tracestart _traceend) (`local.L_Hit`) (`self.GetInstigatorController`) (`local.L_DamageCauser`))
          (return true))
        (:`Is Not Valid`
          (return false))))))

(fn `PickUp`
  (params (Character :type "/Game/SRV_Polygon/Blueprints/Character/BP_BaseCharacter Object Reference"))
  (returns (Success :type Boolean))
  (bind _asbp_player_controller (cast `/Game/SRV_Polygon/Blueprints/Character/BP_PlayerController` (`Pawn.GetController` Character)))
  (`/Game/SRV_Polygon/Blueprints/Equipment/InventoryManagerComponent.AddWeaponToInventory` (`/Game/SRV_Polygon/Blueprints/Character/BP_PlayerController.InventoryManagerComponent` _asbp_player_controller) self Character)
  (return true))

(fn `Shoot`
  (`KismetSystemLibrary.PrintString` "Shoot"))

(fn `UserConstructionScript`
  (`parent.UserConstructionScript`))

(fn `UseWeapon`
  (params (Use :type Boolean))
  (returns (Used :type Boolean))
  (if Use
    (if (`self.IsAbleToUse`)
      (set `self.WeaponCanBeUse?` false)
      (`self.Shoot`)
      (if (`self.AutoFire`)
        (set `self.Firing` true)
        (return true)
        (else
          (return true))))
    (else
      (set `self.Firing` false)
      (return false))))

(fn `WeaponTimer`
  (if (not (`self.WeaponCanBeUse?`))
    (bind _output_get (set `self.WeaponUseTiming` (+ (`self.WeaponUseTiming`) (`GameplayStatics.GetWorldDeltaSeconds`))))
    (if (>= _output_get (/ 1.0 (`self.UsePerSecond`)))
      (set `self.WeaponCanBeUse?` true)
      (set `self.WeaponUseTiming` 0.0))))