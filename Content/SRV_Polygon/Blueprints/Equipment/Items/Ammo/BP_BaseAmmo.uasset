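; Base ammo pickup actor that grants ammo of a configured type and amount to the player.
; The Construction Script selects the static mesh from the ammo type, covering pistol, rifle, sniper and grenade launcher.
; When a pawn controlled by BP_PlayerController overlaps the box, a DoOnce-guarded step adds the ammo through that controller's InventoryManagerComponent, then destroys the pickup.
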(event `self.Box.OnComponentBeginOverlap`
  (params (OverlappedComponent :type "PrimitiveComponent Object Reference") (OtherActor :type "Actor Object Reference") (OtherComp :type "PrimitiveComponent Object Reference") (OtherBodyIndex :type Integer) (bFromSweep :type Boolean) (SweepResult :type "HitResult Structure (by ref)"))
  (bind _aspawn (cast `Pawn` OtherActor))
  (bind _asbp_player_controller (cast `/Game/SRV_Polygon/Blueprints/Character/BP_PlayerController` (`Pawn.GetController` _aspawn)))
  (`/Engine/EditorBlueprintResources/StandardMacros.DoOnce` false
    (:`Completed`
      (`/Game/SRV_Polygon/Blueprints/Equipment/InventoryManagerComponent.Add Ammo` (`/Game/SRV_Polygon/Blueprints/Character/BP_PlayerController.InventoryManagerComponent` _asbp_player_controller) (`self.AmmoType`) (`self.AmmoToAdd`))
      (`self.K2_DestroyActor`))))

(fn `UserConstructionScript`
  (`parent.UserConstructionScript`)
  (switch `/Game/SRV_Polygon/Blueprints/Equipment/Items/Ammo/E_AmmoType` (`self.AmmoType`)
    (:`NewEnumerator0`
      (`StaticMeshComponent.SetStaticMesh` (`self.StaticMesh`) "/Game/SRV_Polygon/Assets/UnchartedLike/MilitaryWeapSilver/Pickups/Pistol_Pickup.Pistol_Pickup"))
    (:`NewEnumerator1`
      (`StaticMeshComponent.SetStaticMesh` (`self.StaticMesh`) "/Game/SRV_Polygon/Assets/UnchartedLike/MilitaryWeapSilver/Pickups/AssaultRifle_Pickup.AssaultRifle_Pickup"))
    (:`NewEnumerator2`
      (`StaticMeshComponent.SetStaticMesh` (`self.StaticMesh`) "/Game/SRV_Polygon/Assets/UnchartedLike/MilitaryWeapSilver/Pickups/SniperRifle_Pickup.SniperRifle_Pickup"))
    (:`NewEnumerator3`
      (`StaticMeshComponent.SetStaticMesh` (`self.StaticMesh`) "/Game/SRV_Polygon/Assets/UnchartedLike/MilitaryWeapSilver/Pickups/GrenadeLauncher_Pickup.GrenadeLauncher_Pickup"))))