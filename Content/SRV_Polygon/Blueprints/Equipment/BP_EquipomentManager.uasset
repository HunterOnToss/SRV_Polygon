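; Equipment manager component for BP_BaseCharacter that lets the owning character pick up items it looks at.
; On BeginPlay it caches the owner as the player.
; PickUp runs CheckItems, a persistently debug-drawn object-type line trace from the follow camera along the controller's forward vector.
; If the hit actor implements I_Interact, it sends that actor the pickup message with the player and prints the result.
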(event `self.ReceiveBeginPlay`
  (bind _asbp_base_character (cast `/Game/SRV_Polygon/Blueprints/Character/BP_BaseCharacter` (`self.GetOwner`)))
  (set `self.Player` _asbp_base_character))

(event `PickUp`
  (bind (_outhit _ishit) (`self.Check Items`))
  (bind (_bblockinghit _binitialoverlap _time _distance _location _impactpoint _normal _impactnormal _physmat _hitactor) (`GameplayStatics.BreakHitResult` _outhit))
  (if _ishit
    (if (`KismetSystemLibrary.DoesImplementInterface` _hitactor "/Game/SRV_Polygon/Blueprints/Equipment/I_Interact.I_Interact_C")
      (bind _success (message `/Game/SRV_Polygon/Blueprints/Equipment/I_Interact.PickUp` _hitactor (`self.Player`)))
      (`KismetSystemLibrary.PrintString` (`KismetStringLibrary.Concat_StrStr` "Pick up is : " (`KismetStringLibrary.Conv_BoolToString` _success))))))

(fn `Check Items`
  (returns (OutHit :type "HitResult Structure") (IsHit :type Boolean))
  (bind _player (`self.Player`))
  (bind _returnvalue (`SceneComponent.K2_GetComponentLocation` (`/Game/SRV_Polygon/Blueprints/Character/BP_BaseCharacter.FollowCamera` _player)))
  (bind (_outhit _returnvalue_2) (`KismetSystemLibrary.LineTraceSingleForObjects` :`Start` _returnvalue :`End` (+ _returnvalue (* (`Actor.GetActorForwardVector` (`Pawn.GetController` _player)) (`self.CheckLenght `))) :`ObjectTypes` (`|MakeArray` "ObjectTypeQuery7" :!type "EObjectTypeQuery Enum") :`DrawDebugType` "Persistent"))
  (return _outhit _returnvalue_2))