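; Inventory component that manages an owner's carried items, weapons, equipped weapon and ammo counts by type.
; Items are frozen, hidden and attached on pickup, while weapons claim a free body socket matching their attach points.
; Drops free the socket and restore physics, placing objects ahead of the player controller's character, or the owner otherwise.
; Weapon and ammo changes fire an inventory update notification; the item capacity check always passes.
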(event `DropWeapon`
  (params (Weapon :type "/Game/SRV_Polygon/Blueprints/Equipment/Items/Weapons/BP_BaseWeapon Object Reference"))
  (set `/Game/SRV_Polygon/Blueprints/Equipment/Items/Weapons/BP_BaseWeapon.IsEquiped` false Weapon)
  (`Actor.SetOwner` Weapon null)
  (`self.DropWeaponToWorld` Weapon)
  (`self.OnInventoryStateUpdate`)
  (if (== Weapon (`self.GetCurrentEquipedWeapon`))
    (`self.ClearEquipedWeapon`)))

(event `EquipWeapon`
  (params (Weapon :type "/Game/SRV_Polygon/Blueprints/Equipment/Items/Weapons/BP_BaseWeapon Object Reference"))
  (`self.SetEquipedWeapon` Weapon)
  (`self.OnInventoryStateUpdate`))

(event `UnEquipWeapon`
  (`self.ClearEquipedWeapon`)
  (`self.OnInventoryStateUpdate`))

(fn `Add Ammo`
  (params (Type :type "/Game/SRV_Polygon/Blueprints/Equipment/Items/Ammo/E_AmmoType Enum" :default "NewEnumerator0") (Amount :type Integer))
  (locals (L_Type :type "/Game/SRV_Polygon/Blueprints/Equipment/Items/Ammo/E_AmmoType Enum" :default "NewEnumerator0") (L_Amount :type Integer) (L_Index :type Integer) (L_UpdateAmmoInfo :type "/Game/SRV_Polygon/Blueprints/Equipment/Items/Ammo/S_AmmoInfo Structure"))
  (set `local.L_Type` Type)
  (set `local.L_Amount` Amount)
  (for (_array_element _array_index) (`self.Ammo`)
    (bind (_ammotype _amount) (break `/Game/SRV_Polygon/Blueprints/Equipment/Items/Ammo/S_AmmoInfo` _array_element))
    (if (`|EnumEquality` _ammotype (`local.L_Type`))
      (set `local.L_Index` _array_index)
      (set `local.L_UpdateAmmoInfo` (make `/Game/SRV_Polygon/Blueprints/Equipment/Items/Ammo/S_AmmoInfo` _ammotype (+ _amount (`local.L_Amount`))))
      (break)))
  (`KismetArrayLibrary.Array_Set` (`self.Ammo`) (`local.L_Index`) (`local.L_UpdateAmmoInfo`))
  (`self.OnInventoryStateUpdate`))

(fn `Add Item to Inventory`
  (params (Item :type "/Game/SRV_Polygon/Blueprints/Equipment/Items/BP_BaseItem Object Reference") (ActorToAttach :type "Actor Object Reference"))
  (returns (Success :type Boolean))
  (locals (L_Item :type "/Game/SRV_Polygon/Blueprints/Equipment/Items/BP_BaseItem Object Reference") (L_ActorToAttach :type "Actor Object Reference"))
  (bind _l_item (`local.L_Item`))
  (bind _output_get (set `local.L_Item` Item))
  (if (`self.CanBeAdded` _output_get)
    (set `local.L_ActorToAttach` ActorToAttach)
    (`KismetArrayLibrary.Array_Add` (`self.InventoryStorageItems`) (`local.L_Item`))
    (`/Game/SRV_Polygon/Blueprints/Equipment/Items/BP_BaseItem.FreezePhysComponents` _l_item true)
    (`Actor.SetActorEnableCollision` _l_item false)
    (`Actor.K2_AttachToActor` _l_item (`local.L_ActorToAttach`) "None" "SnapToTarget" "SnapToTarget" "KeepRelative" true)
    (`Actor.SetActorHiddenInGame` (`local.L_Item`) true)
    (else
      (return false))))

(fn `AddWeaponToInventory`
  (params (Weapon :type "/Game/SRV_Polygon/Blueprints/Equipment/Items/Weapons/BP_BaseWeapon Object Reference") (Character :type "Actor Object Reference"))
  (locals (L_Weapon :type "/Game/SRV_Polygon/Blueprints/Equipment/Items/Weapons/BP_BaseWeapon Object Reference"))
  (bind _output_get (set `local.L_Weapon` Weapon))
  (`Actor.SetOwner` _output_get Character)
  (`KismetArrayLibrary.Array_Add` (`self.InventoryWeaponItems`) _output_get)
  (bind (_freepoint _found_) (`self.FindFreeSocket` (`local.L_Weapon`)))
  (if _found_
    (`self.MarkSocketAsUse` _freepoint (`local.L_Weapon`))
    (`/Game/SRV_Polygon/Blueprints/Equipment/Items/BP_BaseItem.FreezePhysComponents` (`local.L_Weapon`) true)
    (`Actor.SetActorEnableCollision` (`local.L_Weapon`) false)
    (`/Game/SRV_Polygon/Blueprints/Equipment/Items/Weapons/BP_BaseWeapon.AttachWeaponToCharacter` (`local.L_Weapon`) (`/Game/SRV_Polygon/Blueprints/Equipment/BP_MyLibs.GetSocketNameByPoint` _freepoint))
    (`self.OnInventoryStateUpdate`)))

(fn `CanBeAdded`
  (params (Item :type "/Game/SRV_Polygon/Blueprints/Equipment/Items/BP_BaseItem Object Reference"))
  (returns (Success :type Boolean))
  (return true))

(fn `ClearEquipedWeapon`
  (set `self.EquipedWeapon` null))

(fn `DropItemToWorld`
  (params (Item :type "/Game/SRV_Polygon/Blueprints/Equipment/Items/BP_BaseItem Object Reference"))
  (locals (L_Item :type "/Game/SRV_Polygon/Blueprints/Equipment/Items/BP_BaseItem Object Reference") (L_DropLocation :type "Vector Structure" :default (0.0 0.0 0.0)))
  (bind _output_get (set `local.L_Item` Item))
  (bind _returnvalue (`self.RemoveItemFromInventory` _output_get))
  (if _returnvalue
    (set `local.L_DropLocation` (`self.DropLocation`))
    (`Actor.K2_SetActorLocation` (`local.L_Item`) (`local.L_DropLocation`) false true)
    (`Actor.SetActorHiddenInGame` (`local.L_Item`) false)
    (`/Game/SRV_Polygon/Blueprints/Equipment/Items/BP_BaseItem.FreezePhysComponents` (`local.L_Item`) false)
    (`Actor.K2_DetachFromActor` (`local.L_Item`) "KeepWorld" "KeepWorld" "KeepWorld")
    (`Actor.SetActorEnableCollision` (`local.L_Item`) true)))

(fn `DropLocation`
  (returns (Location :type "Vector Structure"))
  (bind _returnvalue (`self.GetOwner`))
  (bind _asbp_player_controller (cast `/Game/SRV_Polygon/Blueprints/Character/BP_PlayerController` _returnvalue)
    (:`then`
      (bind _characterreference (`/Game/SRV_Polygon/Blueprints/Character/BP_PlayerController.CharacterReference` _asbp_player_controller))
      (return (+ (`Actor.K2_GetActorLocation` _characterreference) (* (`Actor.GetActorForwardVector` _characterreference) (`self.DropDistance`)))))
    (:`CastFailed`
      ;[1 1 1] На тот случай если владелец не будет игроком.
      (return (+ (`Actor.K2_GetActorLocation` _returnvalue) (* (`Actor.GetActorForwardVector` _returnvalue) (`self.DropDistance`)))))))

(fn `DropWeaponToWorld`
  (params (Weapon :type "/Game/SRV_Polygon/Blueprints/Equipment/Items/Weapons/BP_BaseWeapon Object Reference"))
  (locals (L_Item :type "/Game/SRV_Polygon/Blueprints/Equipment/Items/BP_BaseItem Object Reference") (L_DropLocation :type "Vector Structure" :default (0.0 0.0 0.0)))
  (bind _output_get (set `local.L_Item` Weapon))
  (`self.Remove Weapon from Inventory` _output_get)
  (set `local.L_DropLocation` (`self.DropLocation`))
  (`Actor.K2_SetActorLocation` (`local.L_Item`) (`local.L_DropLocation`) false true)
  (`/Game/SRV_Polygon/Blueprints/Equipment/Items/BP_BaseItem.FreezePhysComponents` (`local.L_Item`) false)
  (`Actor.K2_DetachFromActor` (`local.L_Item`) "KeepWorld" "KeepWorld" "KeepWorld")
  (`Actor.SetActorEnableCollision` (`local.L_Item`) true)
  (`Actor.SetActorHiddenInGame` (`local.L_Item`) false))

(fn `FindFreeSocket`
  (params (ForWeapon :type "/Game/SRV_Polygon/Blueprints/Equipment/Items/Weapons/BP_BaseWeapon Object Reference"))
  (returns (FreePoint :type "/Game/SRV_Polygon/Blueprints/Equipment/E_AttachPoint Enum") (`Found?` :type Boolean))
  (locals (L_FoundSocket :type Boolean) (L_SocketPoint :type "/Game/SRV_Polygon/Blueprints/Equipment/E_AttachPoint Enum"))
  (for _array_element (`/Game/SRV_Polygon/Blueprints/Equipment/Items/Weapons/BP_BaseWeapon.AttachPoints` ForWeapon)
    (for _array_element_2 (`self.SocketStates`)
      (bind (_inuse _attachtype) (break `/Game/SRV_Polygon/Blueprints/Equipment/S_AttachInfo` _array_element_2))
      (if (and (`|EnumEquality` _array_element _attachtype) (not _inuse))
        (set `local.L_FoundSocket` true)
        (set `local.L_SocketPoint` _array_element))))
  (return (`local.L_SocketPoint`) (`local.L_FoundSocket`)))

(fn `GetCurrentAmmo`
  (params (ForType :type "/Game/SRV_Polygon/Blueprints/Equipment/Items/Ammo/E_AmmoType Enum" :default "NewEnumerator0"))
  (returns (Ammo :type Integer))
  (for _array_element (`self.Ammo`)
    (bind (_ammotype _amount) (break `/Game/SRV_Polygon/Blueprints/Equipment/Items/Ammo/S_AmmoInfo` _array_element))
    (if (`|EnumEquality` _ammotype ForType)
      (return _amount))))

(fn `GetCurrentEquipedWeapon`
  (returns (EquipedWeapon :type "/Game/SRV_Polygon/Blueprints/Equipment/Items/Weapons/BP_BaseWeapon Object Reference"))
  (return (`self.EquipedWeapon`)))

(fn `GetSocketByName`
  (params (Type :type "/Game/SRV_Polygon/Blueprints/Equipment/E_AttachPoint Enum" :default "NewEnumerator0"))
  (returns (Name :type Name))
  (switch `/Game/SRV_Polygon/Blueprints/Equipment/E_AttachPoint` Type
    (:`NewEnumerator0`
      (return "S_Left"))
    (:`NewEnumerator1`
      (return "S_Right"))
    (:`NewEnumerator2`
      (return "S_Back"))
    (:`NewEnumerator3`
      (return "S_BackSecond"))))

(fn `MarkSocketAsAvailable`
  (params (Point :type "/Game/SRV_Polygon/Blueprints/Equipment/E_AttachPoint Enum" :default "NewEnumerator0"))
  (locals (L_Index :type Integer) (L_NewAttachInfo :type "/Game/SRV_Polygon/Blueprints/Equipment/S_AttachInfo Structure"))
  (for (_array_element _array_index) (`self.SocketStates`)
    (bind (_inuse _attachtype) (break `/Game/SRV_Polygon/Blueprints/Equipment/S_AttachInfo` _array_element))
    (if (`|EnumEquality` _attachtype Point)
      (set `local.L_Index` _array_index)
      (set `local.L_NewAttachInfo` (make `/Game/SRV_Polygon/Blueprints/Equipment/S_AttachInfo` false _attachtype))
      (break)))
  (`KismetArrayLibrary.Array_Set` (`self.SocketStates`) (`local.L_Index`) (`local.L_NewAttachInfo`)))

(fn `MarkSocketAsUse`
  (params (Point :type "/Game/SRV_Polygon/Blueprints/Equipment/E_AttachPoint Enum" :default "NewEnumerator0") (WeaponRef :type "/Game/SRV_Polygon/Blueprints/Equipment/Items/Weapons/BP_BaseWeapon Object Reference"))
  (locals (L_Index :type Integer) (L_NewAttachInfo :type "/Game/SRV_Polygon/Blueprints/Equipment/S_AttachInfo Structure"))
  (for (_array_element _array_index) (`self.SocketStates`)
    (bind (_inuse _attachtype) (break `/Game/SRV_Polygon/Blueprints/Equipment/S_AttachInfo` _array_element))
    (if (`|EnumEquality` _attachtype Point)
      (set `local.L_Index` _array_index)
      (set `local.L_NewAttachInfo` (make `/Game/SRV_Polygon/Blueprints/Equipment/S_AttachInfo` true _attachtype WeaponRef))
      (break)))
  (`KismetArrayLibrary.Array_Set` (`self.SocketStates`) (`local.L_Index`) (`local.L_NewAttachInfo`)))

(fn `Remove Weapon from Inventory`
  (params (Weapon :type "/Game/SRV_Polygon/Blueprints/Equipment/Items/BP_BaseItem Object Reference"))
  (`KismetArrayLibrary.Array_RemoveItem` (`self.InventoryWeaponItems`) Weapon)
  (for _array_element (`self.SocketStates`)
    (bind (_inuse _attachtype _weaponref) (break `/Game/SRV_Polygon/Blueprints/Equipment/S_AttachInfo` _array_element))
    (if (== _weaponref Weapon)
      (`self.MarkSocketAsAvailable` _attachtype))))

(fn `RemoveItemFromInventory`
  (params (Item :type "/Game/SRV_Polygon/Blueprints/Equipment/Items/BP_BaseItem Object Reference"))
  (returns (ReturnValue :type Boolean))
  (bind _returnvalue (`KismetArrayLibrary.Array_RemoveItem` (`self.InventoryStorageItems`) Item))
  (return _returnvalue))

(fn `SetEquipedWeapon`
  (params (Weapon :type "/Game/SRV_Polygon/Blueprints/Equipment/Items/Weapons/BP_BaseWeapon Object Reference"))
  (set `self.EquipedWeapon` Weapon))