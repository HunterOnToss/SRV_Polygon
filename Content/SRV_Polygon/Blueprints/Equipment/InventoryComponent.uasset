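; InventoryComponent is an equipment component that stores items in an Inventory array.
; InitInventory clears the array, adds one entry for each slot up to the given Size, and always returns true.
; AddItem appends the item to the end and returns its index, with no capacity or free-slot check.
; The event graph has no active logic.
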(fn `AddItem`
  (params (Item :type "/Game/SRV_Polygon/Blueprints/Equipment/BP_BaseItem Object Reference"))
  (returns (Place :type Integer))
  (bind _returnvalue (`KismetArrayLibrary.Array_Add` (`self.Inventory`) Item))
  (return _returnvalue))

(fn `InitInventory`
  (params (Size :type Integer))
  (returns (Success :type Boolean))
  (`KismetArrayLibrary.Array_Clear` (`self.Inventory`))
  (for _ (range Size)
    (`KismetArrayLibrary.Array_Add` (`self.Inventory`)))
  (return true))