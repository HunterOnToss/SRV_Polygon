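; BP_EquipmentManager is an unfinished equipment component that keeps a list of item actors for its owner.
; Items are added and removed directly, though AddItem and CanBeAdded always return false.
; Dropping removes an item and teleports it in front of the owner, but sets it hidden.
; Physics freezing around the drop is an empty stub, and the scan caching simulating components is never called here.
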(fn `AddItem`
  (params (Item :type "/Game/SRV_Polygon/Blueprints/Equipment/BP_BaseItem Object Reference"))
  (returns (Success :type Boolean))
  (`KismetArrayLibrary.Array_Add` (`self.Items`) Item)
  (return false))

(fn `CanBeAdded`
  (params (Item :type "/Game/SRV_Polygon/Blueprints/Equipment/BP_BaseItem Object Reference"))
  (returns (Success :type Boolean))
  (return false))

(fn `DropItemToWorld`
  (params (Item :type "/Game/SRV_Polygon/Blueprints/Equipment/BP_BaseItem Object Reference"))
  (locals (L_Item :type "/Game/SRV_Polygon/Blueprints/Equipment/BP_BaseItem Object Reference"))
  (bind _output_get (set `local.L_Item` Item))
  (bind _returnvalue (`self.RemoveItem` _output_get))
  (if _returnvalue
    (`self.FreezePhysComponents` true)
    (`Actor.K2_SetActorLocation` (`local.L_Item`) (`self.DropLocation`) false true)
    (`Actor.SetActorHiddenInGame` (`local.L_Item`) true)
    (`self.FreezePhysComponents` false)))

(fn `DropLocation`
  (returns (Location :type "Vector Structure"))
  (bind _returnvalue (`self.GetOwner`))
  (return (+ (`Actor.K2_GetActorLocation` _returnvalue) (* (`Actor.GetActorForwardVector` _returnvalue) (`self.DropDistance`)))))

(fn `FreezePhysComponents`
  (params (Freeze :type Boolean)))

(fn `RemoveItem`
  (params (Item :type "/Game/SRV_Polygon/Blueprints/Equipment/BP_BaseItem Object Reference"))
  (returns (ReturnValue :type Boolean))
  (bind _returnvalue (`KismetArrayLibrary.Array_RemoveItem` (`self.Items`) Item))
  (return _returnvalue))

(fn `ScanForPhyscComponents`
  (params (Item :type "/Game/SRV_Polygon/Blueprints/Equipment/BP_BaseItem Object Reference"))
  (locals (L_Components :type "Array of PrimitiveComponent Object Reference"))
  (bind _output_get (set `local.L_Components` (`Actor.K2_GetComponentsByClass` Item "/Script/Engine.PrimitiveComponent")))
  (for _array_element _output_get
    (if (`SceneComponent.IsSimulatingPhysics` _array_element "None")
      (`KismetArrayLibrary.Array_Add` (`self.PhysComponents`) _array_element))))